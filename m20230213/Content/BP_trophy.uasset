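; BP_trophy is a trophy object that continuously spins and bobs up and down.
; Each Tick it applies a small world rotation to its Sphere component and moves it along relative Z.
; The IsMoveUp flag reverses direction at fixed upper and lower height limits.
; Steps are fixed per frame without delta-time scaling, so the speed depends on frame rate.
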(event `self.ReceiveTick`
  (params (DeltaSeconds :type "Float (single-precision)"))
  (bind _sphere (`self.Sphere`))
  (bind _sphere_2 (`self.Sphere`))
  (bind (_relativelocation_x _relativelocation_y _relativelocation_z) (`KismetMathLibrary.BreakVector` (`SceneComponent.RelativeLocation` _sphere)))
  (bind (_relativelocation_x_2 _relativelocation_y_2 _relativelocation_z_2) (`KismetMathLibrary.BreakVector` (`SceneComponent.RelativeLocation` _sphere_2)))
  ;[0 1 0.2961] 회전
  (`SceneComponent.K2_AddWorldRotation` (`self.Sphere`) (struct :`Yaw` 1.0) false false)
  (if (`self.IsMoveUp`)
    ;[1 0.1667 0.1667] 위로 이동
    (`SceneComponent.K2_AddRelativeLocation` _sphere_2 (0.0 0.0 1.0) false false)
    (if (>= _relativelocation_z_2 200.0)
      (set `self.IsMoveUp` false))
    (else
      ;[0.2276 0.87 1] 아래로 이동
      (`SceneComponent.K2_AddRelativeLocation` _sphere (`KismetMathLibrary.MakeVector` 0.0 0.0 (* 1.0 -1.0)) false false)
      (if (< _relativelocation_z 0.0)
        (set `self.IsMoveUp` true)))))

(fn `UserConstructionScript`)